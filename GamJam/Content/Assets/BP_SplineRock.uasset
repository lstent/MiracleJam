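; BP_SplineRock is a construction-time Blueprint that adds spline mesh components based on a spline's point count.
; The construction script adds one component per spline segment, attaches it to DefaultSceneRoot and gives it a random world rotation without roll.
; The components never receive spline locations or tangents, as those lookups are unconnected.
; The event graph holds only disabled placeholder events, so it adds no runtime logic.
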(event EventBeginPlay)

(event Collision|EventActorBeginOverlap
  (params (OtherActor :type Actor%20Object%20Reference)))

(event EventTick
  (params (DeltaSeconds :type Float%20%28single-precision%29)))

(fn ConstructionScript
  (for _index (range 0 (- (Spline|GetNumberOfSplinePoints (Variables|Default|GetSpline)) 2))
    (bind _returnvalue (AddComponent|AddSplineMeshComponent false))
    (Transformation|AttachComponentToComponent _returnvalue (Variables|Default|GetDefaultSceneRoot) "None" "KeepRelative" "KeepRelative" "KeepRelative" true)
    (Transformation|SetWorldRotation _returnvalue (Math|Random|RandomRotator false) false false)))