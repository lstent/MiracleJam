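; Sun projectile actor in the collectables set that can be consumed or fizzle out after bouncing.
; The Boucy component's hit event tolerates one impact through a HitOnce flag, then calls DestroyProjectile on the next.
; ConsumeProjectile and DestroyProjectile play Collect or Fizzle respectively, then share cleanup that stops the main Niagara effect, removes Boucy and Sphere, and sets a short lifespan.
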(event OnComponentHit(Boucy)
  (params (HitComponent :type Primitive%20Component%20Object%20Reference) (OtherActor :type Actor%20Object%20Reference) (OtherComp :type Primitive%20Component%20Object%20Reference) (NormalImpulse :type Vector :default "0, 0, 0") (Hit :type Hit%20Result%20Structure%20%28by%20ref%29))
  (if (Variables|Default|GetHitOnce)
    (CallFunction|DestroyProjectile)
    (else
      (Variables|Default|SetHitOnce true))))

(event Custom|DestroyProjectile
  (Components|Activation|Activate (Variables|Default|GetFizzle) false)
  (Components|Activation|Deactivate (Variables|Default|GetNiagara1))
  (Components|DestroyComponent (Variables|Default|GetBoucy))
  (Actor|SetLifeSpan 1.0))

(event Custom|Consume%20Projectile
  (Components|Activation|Activate (Variables|Default|GetCollect) false)
  (Components|Activation|Deactivate (Variables|Default|GetNiagara1))
  (Components|DestroyComponent (Variables|Default|GetBoucy))
  (Actor|SetLifeSpan 1.0))

(event EventBeginPlay)

(event Collision|EventActorBeginOverlap
  (params (OtherActor :type Actor%20Object%20Reference)))

(event EventTick
  (params (DeltaSeconds :type Float%20%28single-precision%29)))

(fn ConstructionScript)