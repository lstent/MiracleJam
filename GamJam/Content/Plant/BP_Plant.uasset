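; BP_Plant is a plant actor that reveals growth tiers as it absorbs collectibles.
; When an actor whose class exactly matches CollectiblesRef overlaps its Capsule, it adds to Score and destroys that actor.
; CheckScore then shows Tier2 through Tier5 at fixed, exact score milestones, without hiding earlier tiers.
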(event OnComponentBeginOverlap(Capsule)
  (params (OverlappedComponent :type Primitive%20Component%20Object%20Reference) (OtherActor :type Actor%20Object%20Reference) (OtherComp :type Primitive%20Component%20Object%20Reference) (OtherBodyIndex :type Integer) (bFromSweep :type Boolean) (SweepResult :type Hit%20Result%20Structure%20%28by%20ref%29))
  (if (== (Variables|Default|GetCollectiblesRef) (Utilities|GetClass OtherActor))
    (Variables|Default|SetScore (+ (Variables|Default|GetScore) 10))
    (Actor|DestroyActor OtherActor)
    (CallFunction|CheckScore)))

(event Custom|CheckScore
  (if (== (Variables|Default|GetScore) 50)
    (Rendering|SetVisibility (Variables|Default|GetTier2) true false)
    (elif (== (Variables|Default|GetScore) 100)
      (Rendering|SetVisibility (Variables|Default|GetTier3) true false)
      (elif (== (Variables|Default|GetScore) 150)
        (Rendering|SetVisibility (Variables|Default|GetTier4) true false)
        (elif (== (Variables|Default|GetScore) 200)
          (Rendering|SetVisibility (Variables|Default|GetTier5) true false))))))

(event EventBeginPlay)

(event Collision|EventActorBeginOverlap
  (params (OtherActor :type Actor%20Object%20Reference)))

(event EventTick
  (params (DeltaSeconds :type Float%20%28single-precision%29)))

(fn ConstructionScript)